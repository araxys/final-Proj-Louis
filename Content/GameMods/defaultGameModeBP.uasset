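; Game mode for a local two-player fighting game that runs timed rounds and tracks the match winner.
; BeginPlay spawns each GameInstance-selected character at P1/P2-tagged PlayerStarts, possesses and cross-links them, sets the camera and HUD, then unlocks movement after a delay.
; ResetMatchVariables clears wins, destroys both fighters and reuses that setup chain.
; While the timer is active, Tick counts down to TimeOver, which awards the round to the healthier player.
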(event `RoundStart`
  (set `self.isTimerActive` true)
  (set `HonorObliterationCharacter.canMove` true (`self.Player1`))
  (set `HonorObliterationCharacter.canMove` true (`self.Player2`))
  (set `HonorObliterationCharacter.playerHealth` 1.0 (`self.Player1`))
  (set `HonorObliterationCharacter.playerHealth` 1.0 (`self.Player2`)))

(event `P1RW`
  (if (< (`HonorObliterationCharacter.playerHealth` (`self.Player2`)) 0.0)
    (`HonorObliterationCharacter.WinRound` (`self.Player1`))
    (set `self.roundTime` 20.0)))

(event `RoundEnd`
  (set `self.isTimerActive` false)
  (set `HonorObliterationCharacter.canMove` false (`self.Player1`))
  (set `HonorObliterationCharacter.canMove` false (`self.Player2`)))

(event `self.ReceiveTick`
  (params (DeltaSeconds :type "Float (single-precision)"))
  (bind _returnvalue (- (`self.roundTime`) DeltaSeconds))
  (if (`self.isTimerActive`)
    (if (>= _returnvalue 0.0)
      (set `self.roundTime` _returnvalue)
      (else
        (set `self.roundTime` 0.0)
        (`self.TimeOver`)))))

(event `ResetMatchVariables`
  (bind _player1 (`self.Player1`))
  (bind _player2 (`self.Player2`))
  (set `HonorObliterationCharacter.roundsWon` 0 (`self.Player1`))
  (set `HonorObliterationCharacter.roundsWon` 0 (`self.Player2`))
  (bind _foundwidgets (`WidgetBlueprintLibrary.GetAllWidgetsOfClass` "/Game/UI/HealthStamina.HealthStamina_C"))
  (bind _output (`|GetArrayItem` _foundwidgets))
  (`/Game/UI/HealthStamina.UpdateRoundCircles` _output 0 0)
  (`/Game/UI/HealthStamina.UpdateRoundCircles` _output 1 0)
  (`self.K2_DestroyActor` (`self.Player1`))
  (`self.K2_DestroyActor` (`self.Player2`))
  (set `self.roundTime` 20.0)
  (bind _asbase_game_instance (cast `BaseGameInstance` (`GameplayStatics.GetGameInstance`) :!label _label))
  (set `self.As Base Game Instance` _asbase_game_instance)
  (bind _outactors (`GameplayStatics.GetAllActorsOfClass` "/Script/Engine.PlayerStart"))
  (for _array_element _outactors
    (`self.SpawnPlayers` _array_element))
  (bind _outactors_2 (`GameplayStatics.GetAllActorsOfClass` "/Game/UI/camera/DefaultCamera.DefaultCamera_C"))
  (`/Game/UI/camera/DefaultCamera.UseCamera` (`|GetArrayItem` _outactors_2))
  (if (`KismetSystemLibrary.IsValid` (`self.Player1`))
    (if (`KismetSystemLibrary.IsValid` (`self.Player2`))
      (set `HonorObliterationCharacter.otherPlayer` _player2 _player1)
      (set `HonorObliterationCharacter.otherPlayer` _player1 _player2)
      (set `HonorObliterationCharacter.isFlipped` true _player2)
      (bind _returnvalue (`|CreateWidget` "/Game/UI/HealthStamina.HealthStamina_C" (`GameplayStatics.GetPlayerController` 0)))
      (`UserWidget.AddToViewport` _returnvalue 0)
      (message `/Game/Librarys/HUDRefInterface.SetHUDReference` (`self.Player1`))
      (message `/Game/Librarys/HUDRefInterface.SetHUDReference` (`self.Player2`))
      (`/Game/UI/HealthStamina.TriggerScreenMessage` _returnvalue)
      (set `HonorObliterationCharacter.canMove` false _player1)
      (set `HonorObliterationCharacter.canMove` false _player2)
      (`KismetSystemLibrary.Delay` 3.0)
      (set `HonorObliterationCharacter.canMove` true _player1)
      (set `HonorObliterationCharacter.canMove` true _player2))))

(event `self.ReceiveBeginPlay`
  (goto _label))

(fn `Determine Winner`
  (returns (winnerIndex :type Integer))
  (if (>= (`HonorObliterationCharacter.roundsWon` (`self.Player1`)) (`self.numRounds`))
    (`HonorObliterationCharacter.WinMatch` (`self.Player1`))
    (return 0)
    (elif (>= (`HonorObliterationCharacter.roundsWon` (`self.Player2`)) (`self.numRounds`))
      (`HonorObliterationCharacter.WinMatch` (`self.Player2`))
      (return 1)
      (else
        (return -1)))))

(fn `DetermineCharacterClass`
  (params (Transform :type "Transform Structure") (Actor :type "Actor Object Reference") (PlayerIndex :type Integer))
  (returns (CharacterReference :type "HonorObliterationCharacter Object Reference"))
  (bind _asbase_game_instance (cast `BaseGameInstance` (`GameplayStatics.GetGameInstance`)))
  (switch `int` PlayerIndex
    (:`0`
      (switch `ECharacterClass` (`BaseGameInstance.characterClassP1` _asbase_game_instance)
        (:`VE_Default`
          _)
        (:`VE_Boss`
          (bind _returnvalue (`|SpawnActorFromClass` "/Game/Boss/MyHonorObliterationPlayer_BP.MyHonorObliterationPlayer_BP_C" Transform "Undefined" "OverrideRootScale" Actor null :!label _label))
          (return _returnvalue))
        (:`VE_Countess`
          (bind _returnvalue_2 (`|SpawnActorFromClass` "/Game/Countess/CountessPlayer_BP.CountessPlayer_BP_C" Transform "Undefined" "OverrideRootScale" Actor null :!label _label_2))
          (return _returnvalue_2))))
    (:`1`
      (switch `ECharacterClass` (`BaseGameInstance.characterClassP2` _asbase_game_instance)
        (:`VE_Default`
          _)
        (:`VE_Boss`
          (goto _label))
        (:`VE_Countess`
          (goto _label_2)))))
  (bind _returnvalue_3 (`|SpawnActorFromClass` "/Game/SideScrollerCPP/Blueprints/SideScrollerCharacter.SideScrollerCharacter_C" Transform "Undefined" "OverrideRootScale" Actor null))
  (return _returnvalue_3))

(fn `SpawnPlayers`
  (params (Object :type "Actor Object Reference"))
  (bind _returnvalue (`self.GetTransform` Object))
  (bind _asplayer_start (cast `PlayerStart` Object))
  (bind _playerstarttag (`PlayerStart.PlayerStartTag` _asplayer_start))
  (if (== "P1" _playerstarttag)
    (bind _characterreference (`self.DetermineCharacterClass` (`self.GetTransform` Object) Object))
    (set `self.Player1` _characterreference)
    (`Controller.Possess` (`GameplayStatics.GetPlayerController` 0) _characterreference)
    (elif (== _playerstarttag "P2")
      (bind _returnvalue_2 (`|SpawnActorFromClass` "/Script/HonorObliteration.MyPlayerController" _returnvalue "Undefined" "OverrideRootScale" null null))
      (bind _characterreference_2 (`self.DetermineCharacterClass` _returnvalue Object 1))
      (set `self.Player2` _characterreference_2)
      (`Controller.Possess` _returnvalue_2 _characterreference_2))))

(fn `TimeOver`
  (if (> (`HonorObliterationCharacter.playerHealth` (`self.Player1`)) (`HonorObliterationCharacter.playerHealth` (`self.Player2`)))
    (`HonorObliterationCharacter.WinRound` (`self.Player1`))
    (set `self.roundTime` 60.0)
    (elif (< (`HonorObliterationCharacter.playerHealth` (`self.Player1`)) (`HonorObliterationCharacter.playerHealth` (`self.Player2`)))
      (`HonorObliterationCharacter.WinRound` (`self.Player2`))
      (set `self.roundTime` 99.0))))

(fn `UserConstructionScript`)

(fn `Win Cond P1`)

(fn `WinCondP2`)