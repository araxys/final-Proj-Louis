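; Countess player character Blueprint for a two-player fighting game, linking the pawn to the game mode, HUD and hurtbox.
; On BeginPlay, after a short delay, it caches the game mode and Player 2 reference, then spawns and attaches a hurtbox actor.
; It forwards P2 keyboard inputs for movement and combat to the other character, so one pawn handles both players' keys.
; Custom events relay round start/end and refresh HUD round icons.
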(event `self.UptdateHUDRoundIcons`
  (bind _hudref (`self.hudRef`)
    (:`then`
      (`/Game/UI/HealthStamina.UpdateRoundIcons` _hudref))
    (:`else`)))

(event `self.notifyRoundEnd`
  (bind _asdefault_game_mode_bp (cast `/Game/GameMods/defaultGameModeBP` (`self.GameModeReference`)))
  (`/Game/GameMods/defaultGameModeBP.RoundEnd` _asdefault_game_mode_bp))

(event `/Game/Librarys/HUDRefInterface.SetHUDReference`
  (bind _foundwidgets (`WidgetBlueprintLibrary.GetAllWidgetsOfClass` "/Game/UI/HealthStamina.HealthStamina_C"))
  (set `self.hudRef` (`|GetArrayItem` _foundwidgets)))

(event `self.notifyRoundStart`
  (bind _asdefault_game_mode_bp (cast `/Game/GameMods/defaultGameModeBP` (`self.GameModeReference`)))
  (`/Game/GameMods/defaultGameModeBP.RoundStart` _asdefault_game_mode_bp))

(event `self.ReceiveBeginPlay`
  (`KismetSystemLibrary.Delay` 0.2)
  (bind _ashonor_obliteration_game_mode (cast `HonorObliterationGameMode` (`GameplayStatics.GetGameMode`)))
  (bind _output_get (set `self.GameModeReference` _ashonor_obliteration_game_mode))
  (bind _player2 (`HonorObliterationGameMode.Player2` _output_get))
  (if (not (== _player2 self))
    (set `self.player2reference` _player2))
  (bind _returnvalue (`|SpawnActorFromClass` "/Game/UI/Hitbox/hurtboxActor_BP.hurtboxActor_BP_C" (`self.GetTransform` (`PawnMovementComponent.GetPawnOwner` (`self.CharacterMovement`))) "Undefined" "OverrideRootScale" null null))
  (bind _output_get_2 (set `self.hurtbox` _returnvalue))
  (`self.K2_AttachToActor` _output_get_2 self "None" "SnapToTarget" "SnapToTarget" "SnapToTarget" true)
  (`self.K2_AttachToActor` _returnvalue self "None" "SnapToTarget" "SnapToTarget" "SnapToTarget" true)
  (`self.SetOwner` _returnvalue self))

(event `InputAction|OpenPauseMEnu`
  (params (Key :type "Key Structure"))
  (:`Pressed`
    (bind _returnvalue (`|CreateWidget` "/Game/UI/ChangeControlsScreen.ChangeControlsScreen_C"))
    (`UserWidget.AddToViewport` _returnvalue 0)))

(event `InputAction|JumpP2`
  (params (Key :type "Key Structure"))
  (bind _player2reference (`self.player2reference`))
  (:`Pressed`
    (`/Engine/EditorBlueprintResources/StandardMacros.IsValid` _player2reference
      (:`Is Valid`
        (`self.P2KeyBoardJump` _player2reference))))
  (:`Released`
    (`/Engine/EditorBlueprintResources/StandardMacros.IsValid` _player2reference
      (:`Is Valid`
        (`self.P2KeyBoardStopJumping` _player2reference)))))

(event `InputAction|attack1P2`
  (params (Key :type "Key Structure"))
  (bind _player2reference (`self.player2reference`))
  (:`Pressed`
    (`/Engine/EditorBlueprintResources/StandardMacros.IsValid` _player2reference
      (:`Is Valid`
        (`self.P2KeyBoardAttack1` _player2reference)))))

(event `InputAction|attack2P2`
  (params (Key :type "Key Structure"))
  (bind _player2reference (`self.player2reference`))
  (:`Pressed`
    (`/Engine/EditorBlueprintResources/StandardMacros.IsValid` _player2reference
      (:`Is Valid`
        (`self.P2KeyBoardAttack2` _player2reference)))))

(event `InputAction|attack3P2`
  (params (Key :type "Key Structure"))
  (bind _player2reference (`self.player2reference`))
  (:`Pressed`
    (`/Engine/EditorBlueprintResources/StandardMacros.IsValid` _player2reference
      (:`Is Valid`
        (`self.P2KeyBoardAttack3` _player2reference)))))

(event `InputAction|attack4P2`
  (params (Key :type "Key Structure"))
  (bind _player2reference (`self.player2reference`))
  (:`Pressed`
    (`/Engine/EditorBlueprintResources/StandardMacros.IsValid` _player2reference
      (:`Is Valid`
        (`self.P2KeyBoardAttack4` _player2reference)))))

(event `InputAction|CrouchP2`
  (params (Key :type "Key Structure"))
  (bind _player2reference (`self.player2reference`))
  (:`Pressed`
    (`/Engine/EditorBlueprintResources/StandardMacros.IsValid` _player2reference
      (:`Is Valid`
        (`self.StartCrouching` _player2reference))))
  (:`Released`
    (`/Engine/EditorBlueprintResources/StandardMacros.IsValid` _player2reference
      (:`Is Valid`
        (`self.StopCrouching` _player2reference)))))

(event `InputAction|BlockP2`
  (params (Key :type "Key Structure"))
  (bind _player2reference (`self.player2reference`))
  (:`Pressed`
    (`/Engine/EditorBlueprintResources/StandardMacros.IsValid` _player2reference
      (:`Is Valid`
        (`self.startBlocking` _player2reference))))
  (:`Released`
    (`/Engine/EditorBlueprintResources/StandardMacros.IsValid` _player2reference
      (:`Is Valid`
        (`self.stopBlocking` _player2reference)))))

(event `InputAxis|MoveRightP2`
  (params (AxisValue :type "Float (single-precision)"))
  (bind _player2reference (`self.player2reference`))
  (`/Engine/EditorBlueprintResources/StandardMacros.IsValid` _player2reference
    (:`Is Valid`
      (`self.P2KeyBoardMoveRight` _player2reference AxisValue))))

(event `InputAction|ExceptionnalAttackP2`
  (params (Key :type "Key Structure"))
  (bind _player2reference (`self.player2reference`))
  (:`Pressed`
    (`/Engine/EditorBlueprintResources/StandardMacros.IsValid` _player2reference
      (:`Is Valid`
        (`self.P2KeyBoardExceptionnalAttack` _player2reference)))))

(fn `UserConstructionScript`)